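; BP_PawnBase is a pawn moved by physics, apparently intended as a base for player-controlled pawns.
; Forward and right axis inputs add force to the static mesh along the camera's forward and right vectors, scaled by MoveSpeed without mass compensation.
; Camera yaw and pitch axes feed controller rotation input.
; The event graph and construction script contain no active logic.
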(event `InputAxis|MoveForward`
  (params (AxisValue :type "Float (single-precision)"))
  (`PrimitiveComponent.AddForce` (`self.StaticMesh`) (* (* (`SceneComponent.GetForwardVector` (`self.Camera`)) AxisValue) (`self.MoveSpeed`)) "None" false))

(event `InputAxis|MoveRight`
  (params (AxisValue :type "Float (single-precision)"))
  (`PrimitiveComponent.AddForce` (`self.StaticMesh`) (* (* (`SceneComponent.GetRightVector` (`self.Camera`)) AxisValue) (`self.MoveSpeed`)) "None" false))

(event `InputAxis|CameraYaw`
  (params (AxisValue :type "Float (single-precision)"))
  (`self.AddControllerYawInput` AxisValue))

(event `InputAxis|CameraPitch`
  (params (AxisValue :type "Float (single-precision)"))
  (`self.AddControllerPitchInput` AxisValue))

(fn `UserConstructionScript`)